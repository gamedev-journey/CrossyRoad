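; BP_FlooerChunk is one floor row in a chicken game, made of left, center and right floor pieces with landing nodes and props.
; Helper functions compute the three floor transforms, spawn landing nodes stepping along X with a water flag, and randomly spawn coins at the current node position.
; Each Tick, it checks whether it lies too far behind the chicken on Y, then destroys its tracked floors, nodes, props and itself.
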(event `self.ReceiveTick`
  (params (DeltaSeconds :type "Float (single-precision)"))
  (`self.Check If Destroy Floor Chuck`))

(fn `Calculate Floor Transform`
  (returns (`Transform Left` :type "Transform Structure") (`Transform Mid` :type "Transform Structure") (`Transform Right` :type "Transform Structure") (`Y Position` :type "Float (double-precision)"))
  (bind _position_y (`self.Position Y`))
  (return (`KismetMathLibrary.MakeTransform` (`KismetMathLibrary.MakeVector` -1800.0 _position_y)) (`KismetMathLibrary.MakeTransform` (`KismetMathLibrary.MakeVector` 0.0 _position_y)) (`KismetMathLibrary.MakeTransform` (`KismetMathLibrary.MakeVector` 1800.0 _position_y)) _position_y))

(fn `Check If Destroy Floor Chuck`
  (bind (_returnvalue_x _returnvalue_y) (`KismetMathLibrary.BreakVector` (`self.K2_GetActorLocation`)))
  (bind _chicken_ref (`self.Chicken Ref`))
  (bind (_returnvalue_x_2 _returnvalue_y_2) (`KismetMathLibrary.BreakVector` (`self.K2_GetActorLocation` _chicken_ref)))
  (if (`KismetSystemLibrary.IsValid` _chicken_ref)
    (if (>= _returnvalue_y (+ _returnvalue_y_2 (`self.Max Distance Backwards From Chicken`)))
      (`self.Destroy Meshes Landing Nodes And Props`)
      (`self.K2_DestroyActor`))))

(fn `Construct Landing Node (Floor Chunk)`
  (params (`Is Water` :type Boolean))
  (bind (_returnvalue_x _returnvalue_y) (`KismetMathLibrary.BreakVector` (`self.K2_GetActorLocation`)))
  (bind _returnvalue (`|SpawnActorFromClass` "/Game/Blueprints/BP_LandingNode.BP_LandingNode_C" (`KismetMathLibrary.MakeTransform` (`KismetMathLibrary.MakeVector` (`self.Current X Position For Landing Node`) _returnvalue_y (`self.Current Z Position For Landing Node`))) "Undefined" "OverrideRootScale" null `Is Water` null))
  (set `self.Current X Position For Landing Node` (+ (`self.Current X Position For Landing Node`) 200.0))
  (`KismetArrayLibrary.Array_Add` (`self.Landing Nodes`) _returnvalue))

(fn `Create Coin Attempt`
  (bind (_returnvalue_x _returnvalue_y) (`KismetMathLibrary.BreakVector` (`self.K2_GetActorLocation`)))
  (if (== (`KismetMathLibrary.RandomInteger` 9) 0)
    (`|SpawnActorFromClass` "/Game/Blueprints/BP_Coin.BP_Coin_C" (`KismetMathLibrary.MakeTransform` (`KismetMathLibrary.MakeVector` (`self.Current X Position For Landing Node`) _returnvalue_y (`self.Current Z Position For Landing Node`))) "Undefined" "OverrideRootScale" null null)))

(fn `Destroy Meshes Landing Nodes And Props`
  (for _array_element (`self.Landing Nodes`)
    (`self.K2_DestroyActor` _array_element))
  (`self.K2_DestroyActor` (`self.Left Floor`))
  (`self.K2_DestroyActor` (`self.Right Floor`))
  (`self.K2_DestroyActor` (`self.Center Floor`))
  (for _array_element_2 (`self.Props Array`)
    (`self.K2_DestroyActor` _array_element_2)))

(fn `UserConstructionScript`)